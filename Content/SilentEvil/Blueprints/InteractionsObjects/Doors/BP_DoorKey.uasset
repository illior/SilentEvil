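; BP_DoorKey is the key-item interaction for a BP_LockedDoorByKey door, which it expects as its parent actor.
; SetKey writes the given key type into the InteractableItems array.
; When an item is used and that array is empty, it calls Complete and re-enables the parent door through CloseDoor.
; Close hides the widget and likewise re-enables the door.
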(event Custom|Close%20Door
  (bind _asbp_locked_door_by_key (Utilities|Casting|CastToBP_LockedDoorByKey (Actor|GetParentActor)))
  (Class|SEInteractableObject|SetEnabled _asbp_locked_door_by_key true))

(event EventItemUse
  (params (InItem :type SE%20Quest%20Item%20Object%20Reference))
  (if (== (Utilities|Array|Length (Variables|Default|GetInteractableItems)) 0)
    (Class|SEInteractableTarget|Complete)
    (CallFunction|CloseDoor)))

(event EventClose
  (Rendering|SetVisibility (Variables|Default|GetWidgetComponent) false false)
  (CallFunction|CloseDoor))

(fn ConstructionScript)

(fn SetKey
  (params (KeyType :type SE%20Quest%20Item%20Object%20Reference))
  (Utilities|Array|SetArrayElem (Variables|Default|GetInteractableItems) 0 KeyType))