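; A door that stays locked until opened through a key interaction matching its KeyType.
; On BeginPlay it passes the key type to two BP_DoorKey child actors and binds their completion events.
; Interacting while locked plays a try-open sound, forwards the pawn to one key actor chosen by approach angle, and disables the door's interaction.
; DoorOpen disables both key actors and clears the locked flag.
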(event Custom|DoorOpen
  (params (ActivatedObject :type SE%20Interactable%20Target%20Object%20Reference) (ActivatedBy :type Pawn%20Object%20Reference))
  (Class|SEInteractableObject|SetEnabled (Variables|Default|GetDoorKey) false)
  (Class|SEInteractableObject|SetEnabled (Variables|Default|GetDoorKey1) false)
  (Variables|Default|SetIsDoorLocked false))

(event EventBeginPlay
  (bind _keytype (Variables|Interaction|GetKeyType))
  (bind _asbp_door_key (Utilities|Casting|CastToBP_DoorKey (Variables|/Script/Engine.ChildActorComponent|GetChildActor (Variables|Default|GetBP_UseDoorKey))))
  (bind _output_get (Variables|Default|SetDoorKey _asbp_door_key))
  (Default|SetKey _output_get _keytype)
  (EventDispatchers|BindEventtoOnComplete (Variables|Default|GetDoorKey) (EventDispatchers|CreateEvent :!event Custom|DoorOpen))
  (bind _asbp_door_key_2 (Utilities|Casting|CastToBP_DoorKey (Variables|/Script/Engine.ChildActorComponent|GetChildActor (Variables|Default|GetBP_UseDoorKey1))))
  (bind _output_get_2 (Variables|Default|SetDoorKey1 _asbp_door_key_2))
  (Default|SetKey _output_get_2 _keytype)
  (EventDispatchers|BindEventtoOnComplete (Variables|Default|GetDoorKey1) (EventDispatchers|CreateEvent :!event Custom|DoorOpen)))

(event EventInteract
  (params (Pawn :type Pawn%20Object%20Reference))
  (bind _doorkey (Variables|Default|GetDoorKey))
  (bind _doorkey1 (Variables|Default|GetDoorKey1))
  (if (Variables|Default|GetIsDoorLocked)
    (Audio|PlaySound2D (Variables|Default|GetTryOpenSound) 1.0 1.0 0.0 0 0)
    (bind _returnvalue (Class|SEBaseDoor|GetAngle (Transformation|GetActorLocation Pawn)))
    (if (< _returnvalue 9e+01)
      (Variables|/Script/SilentEvil.SEInteractableObject|SetCurrentPawn _doorkey Pawn)
      (Class|SEInteractableTarget|Interact _doorkey Pawn)
      (else
        (Variables|/Script/SilentEvil.SEInteractableObject|SetCurrentPawn _doorkey1 Pawn)
        (Class|SEInteractableTarget|Interact _doorkey1 Pawn)))
    (Class|SEInteractableObject|SetEnabled false)
    (else
      (CallFunction|PlaySound))))

(fn ConstructionScript)