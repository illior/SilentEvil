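; BP_LockedDoor is an interactable door in SilentEvil that can only be unlocked from one side.
; On Interact, an angle check on the pawn's location decides the side: below 90 degrees clears the locked flag, otherwise it plays a sound.
; Both locked outcomes show a timed help message through the player's SEGameHUD.
; Once unlocked, Interact only calls PlaySound, with no door movement in this graph.
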(event EventInteract
  (params (Pawn :type Pawn%20Object%20Reference))
  (if (Variables|Default|GetIsDoorLocked)
    (if (< (Class|SEBaseDoor|GetAngle (Transformation|GetActorLocation Pawn)) 9e+01)
      (Variables|Default|SetIsDoorLocked false)
      (bind _asplayer_controller (Utilities|Casting|CastToPlayerController (Pawn|GetController Pawn)))
      (bind _assegame_hud (Utilities|Casting|CastToSEGameHUD (HUD|GetHUD _asplayer_controller)))
      (Class|SEGameHUD|ShowHelpText _assegame_hud "You opened it" 2.0)
      (else
        (CallFunction|PlaySound)
        (bind _asplayer_controller_2 (Utilities|Casting|CastToPlayerController (Pawn|GetController Pawn)))
        (bind _assegame_hud_2 (Utilities|Casting|CastToSEGameHUD (HUD|GetHUD _asplayer_controller_2)))
        (Class|SEGameHUD|ShowHelpText _assegame_hud_2 "The door is closed on the other side" 2.0)))
    (else
      (CallFunction|PlaySound))))

(fn ConstructionScript)