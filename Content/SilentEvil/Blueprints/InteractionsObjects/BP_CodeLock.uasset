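; Keypad code lock interaction object that completes when the entered code matches the correct one.
; Move events step a grid cursor across twelve button meshes, swapping materials to highlight the selected key.
; Apply either backspaces, submits or writes the digit read from that button's child text component into the code array, which feeds the display text.
; Submitting compares the code string, calling Complete on a match and resetting the entry either way.
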(event EventMoveHorizontal
  (params (Value :type Float%20%28single-precision%29%20%28by%20ref%29))
  ;[1 1 1] HorizontalMovement
  (if (and (>= (+ Value (.x (Variables|Default|GetCursorPosition))) 0) (< (+ Value (.x (Variables|Default|GetCursorPosition))) (.x (Variables|Default|GetSize))))
    (bind _index (CallFunction|GetIndexbyPosition))
    (Rendering|Material|SetMaterial (Utilities|Array|Get(acopy) (Variables|Default|GetButtons) _index) 0 (Variables|Default|GetDefaultButtonMaterial))
    (Variables|Default|SetCursorPosition (Utilities|Struct|MakeIntPoint (+ (.x (Variables|Default|GetCursorPosition)) Value) (.y (Variables|Default|GetCursorPosition))))
    (bind _index_2 (CallFunction|GetIndexbyPosition))
    (Rendering|Material|SetMaterial (Utilities|Array|Get(acopy) (Variables|Default|GetButtons) _index_2) 0 (Variables|Default|GetActiveButtonMaterial))))

(event EventMoveVertical
  (params (Value :type Float%20%28single-precision%29%20%28by%20ref%29))
  (bind _returnvalue (* Value -1.0))
  ;[1 1 1] VerticalMovement
  (if (and (>= (+ _returnvalue (.y (Variables|Default|GetCursorPosition))) 0) (< (+ _returnvalue (.y (Variables|Default|GetCursorPosition))) (.y (Variables|Default|GetSize))))
    (bind _index (CallFunction|GetIndexbyPosition))
    (Rendering|Material|SetMaterial (Utilities|Array|Get(acopy) (Variables|Default|GetButtons) _index) 0 (Variables|Default|GetDefaultButtonMaterial))
    (Variables|Default|SetCursorPosition (Utilities|Struct|MakeIntPoint (.x (Variables|Default|GetCursorPosition)) (+ (.y (Variables|Default|GetCursorPosition)) _returnvalue)))
    (bind _index_2 (CallFunction|GetIndexbyPosition))
    (Rendering|Material|SetMaterial (Utilities|Array|Get(acopy) (Variables|Default|GetButtons) _index_2) 0 (Variables|Default|GetActiveButtonMaterial))))

(event EventApply
  (bind _index (CallFunction|GetIndexbyPosition))
  (if (== _index 9)
    (|Backspace)
    (elif (== _index 11)
      (|AcceptCode)
      (else
        (|SetNumber _index)))))

(event EventInteract
  (params (Pawn :type Pawn%20Object%20Reference))
  ;[1 1 1] Interact
  (Utilities|FlowControl|Delay 0.11)
  (Rendering|Material|SetMaterial (Utilities|Array|Get(acopy) (Variables|Default|GetButtons)) 0 (Variables|Default|GetActiveButtonMaterial))
  (Variables|Default|SetCursorPosition (Utilities|Struct|MakeIntPoint 0 0)))

(event EventBeginPlay
  (|CreateArray))

(event EventClose
  ;[1 1 1] Close
  (bind _index (CallFunction|GetIndexbyPosition))
  (Rendering|Material|SetMaterial (Utilities|Array|Get(acopy) (Variables|Default|GetButtons) _index) 0 (Variables|Default|GetDefaultButtonMaterial))
  (CallFunction|ResetText))

(fn ConstructionScript)

(fn GetIndexbyPosition
  (bind _cursorposition (Variables|Default|GetCursorPosition))
  (return (+ (.x _cursorposition) (* (.x (Variables|Default|GetSize)) (.y _cursorposition)))))

(fn SetTextCode
  (Variables|Default|SetStringCode "")
  (for _array_element (Variables|Default|GetCurrentCode)
    (Variables|Default|SetStringCode (Utilities|String|Append (Variables|Default|GetStringCode) (Utilities|String|ToString(Integer) _array_element))))
  (Rendering|Components|TextRender|SetText (Variables|Default|GetMainText) (Utilities|Text|ToText(String) (Variables|Default|GetStringCode))))

(fn ResetText
  (bind _currentcode (Variables|Default|GetCurrentCode))
  (for (_ _array_index) _currentcode
    (Utilities|Array|SetArrayElem _currentcode _array_index 0))
  (Variables|Default|SetCurrentIndex 0)
  (CallFunction|SetTextCode))

(fn Success
  (Class|SEInteractableTarget|Complete)
  (bind _index (CallFunction|GetIndexbyPosition))
  (Rendering|Material|SetMaterial (Utilities|Array|Get(acopy) (Variables|Default|GetButtons) _index) 0 (Variables|Default|GetDefaultButtonMaterial))
  (CallFunction|ResetText))

(fn Fail
  (CallFunction|ResetText)
  (Variables|Default|SetCurrentIndex 0))