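; Base interaction target that shows a key prompt through a WBP_Interact widget component when the player is close enough to interact.
; The prompt starts hidden, and StartCanInteract and StopCanInteract toggle a ShowKey flag.
; While the flag is set, Tick shows the key only when the SECharacter camera is within DistanceToInteract of the target location.
; StopCanInteract only clears the flag and does not itself hide the key.
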(event EventBeginPlay
  (bind _aswbp_interact (Utilities|Casting|CastToWBP_Interact (UserInterface|GetUserWidgetObject (Variables|Default|GetWidgetComponent))))
  (Default|SetVisibleKey _aswbp_interact false))

(event EventStartCanInteract
  (params (Pawn :type Pawn%20Object%20Reference))
  (Variables|Default|SetShowKey true))

(event EventStopCanInteract
  (params (Pawn :type Pawn%20Object%20Reference))
  (Variables|Default|SetShowKey false))

(event EventTick
  (params (DeltaSeconds :type Float%20%28single-precision%29))
  (if (Variables|Default|GetShowKey)
    (bind _aswbp_interact (Utilities|Casting|CastToWBP_Interact (UserInterface|GetUserWidgetObject (Variables|Default|GetWidgetComponent))))
    (bind _distance (CallFunction|GetDistance))
    (Default|SetVisibleKey _aswbp_interact (< _distance (Variables|Default|GetDistanceToInteract)))))

(fn ConstructionScript)

(fn GetDistance
  (bind _assecharacter (Utilities|Casting|CastToSECharacter (Variables|Default|GetCurrentPawn))
    (:then
      (return (Math|Vector|Distance(Vector) (Class|SEInteractableObject|GetTargetLocation 0) (Transformation|GetWorldLocation (Variables|/Script/SilentEvil.SECharacter|GetCameraComponent _assecharacter)))))
    (:CastFailed
      (return 1e+03))))