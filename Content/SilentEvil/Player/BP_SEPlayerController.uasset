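; Player controller Blueprint for SilentEvil that binds Alt+number shortcuts, apparently for debugging.
; Alt+1 saves to slot "1" through SEGameModeBase, Alt+2 opens the main menu level, and Alt+3 prints the current level name.
; Disconnected leftovers include a save-slot print and several date-time string formatting nodes; the construction script is empty.
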(event Input|KeyboardEvents|Alt2
  (params (Key :type Key%20Structure :default "None"))
  (:Pressed
    (Game|OpenLevel(byObjectReference) "/Game/SilentEvil/Maps/MainMenu.MainMenu")))

(event Input|KeyboardEvents|Alt1
  (params (Key :type Key%20Structure :default "None"))
  (:Pressed
    (bind _assegame_mode_base (Utilities|Casting|CastToSEGameModeBase (Game|GetGameMode)))
    (Class|SEGameModeBase|SaveGametoSlot _assegame_mode_base (Utilities|String|ToString(Name) "1"))))

(event Input|KeyboardEvents|Alt3
  (params (Key :type Key%20Structure :default "None"))
  (:Pressed
    (bind _returnvalue (Game|GetCurrentLevelName true))
    (Development|PrintString _returnvalue)))

(fn ConstructionScript)